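; Spawner manager that places carrots at random free item spawner points in the level.
; Two seconds after BeginPlay, SRV_spawnCarrot gathers all Bp_itemSpawner actors and, for each pending carrot, picks a random unoccupied one and stores the new carrot on it.
; Successful spawns are subtracted from CarrotAmount, and a Dutch debug message prints the remainder.
; A Reloop event repeats the delayed spawn while carrots remain, though nothing here calls it.
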(event Custom|SRV_spawnCarrot
  (bind _outactors (Actor|GetAllActorsOfClass "/Game/actorReleted/bp_masterItem/bp_itemSpawner.bp_itemSpawner_C"))
  (Variables|Default|SetspawnerList _outactors)
  (Utilities|FlowControl|ForLoopwithBreak 0 (- (Variables|CarrotSettings|GetcarrotAmount) 1)
    (:LoopBody
      (bind _availablespawner (Utilities|CheckAvailableSpawners)
        (:foundAvailableSlot
          (bind _output_get (Variables|Default|SetAvailableSpawner _availablespawner))
          (bind _returnvalue (Game|SpawnActorfromClass "/Game/actorReleted/bp_masterItem/bp_carrot.bp_carrot_C" (Math|Transform|MakeTransform (Transformation|GetActorLocation _output_get) "0, 0, 0" "1,1,1") "AdjustIfPossibleButAlwaysSpawn" 0 0))
          (Variables|/Game/actorReleted/bp_masterItem/bp_itemSpawner.bp_itemSpawner_C|SetBP_Item _output_get _returnvalue))))
    (:Completed
      (Variables|CarrotSettings|SetcarrotAmount (- (Variables|CarrotSettings|GetcarrotAmount) (Variables|Default|GetAmountToRemove)))
      (Development|PrintString (Utilities|String|Append "Je moet nog " (Utilities|String|ToString(Integer) (Variables|CarrotSettings|GetcarrotAmount)) " carrot spawnen") true true "(R=0.000000,G=0.660000,B=1.000000,A=1.000000)" 8.0))))

(event Custom|Reloop
  (if (not (== (Variables|CarrotSettings|GetcarrotAmount) 0))
    (Variables|Default|SetAmountToRemove 0)
    (Utilities|FlowControl|Delay 2.0)
    (CallFunction|SRVSpawnCarrot)))

(event EventBeginPlay
  (Utilities|FlowControl|Delay 2.0)
  (CallFunction|SRVSpawnCarrot))

(fn ConstructionScript)